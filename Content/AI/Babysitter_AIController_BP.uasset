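; AI controller Blueprint for the babysitter character that starts its behavior tree.
; On BeginPlay it casts the controlled pawn to Babysitter_BP, stores it, and sets up the Babysitter_Board blackboard.
; It writes the locations of the pawn's in-room and start point actors as RoomPoint and HallPoint, then runs Babysitter_BT.
; The SetIsNaughty event is declared but has no logic.
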(event Custom|SetIsNaughty
  (params (IsNaughty :type Boolean)))

(event EventBeginPlay
  (bind _self self)
  (bind _returnvalue (AI|GetBlackboard _self))
  (bind _asbabysitter_bp (Utilities|Casting|CastToBabysitter_BP (Pawn|GetControlledPawn)))
  (Variables|Default|SetBabysitterObject _asbabysitter_bp)
  (Class|AIController|UseBlackboard "/Game/AI/Babysitter_Board.Babysitter_Board")
  (AI|Components|Blackboard|SetValueasVector _returnvalue (Utilities|Name|MakeLiteralName "RoomPoint") (Transformation|GetActorLocation (Variables|/Game/Blueprints/Babysitter_BP.Babysitter_BP_C|GetInRoomPoint (Variables|Default|GetBabysitterObject))))
  (AI|Components|Blackboard|SetValueasVector _returnvalue (Utilities|Name|MakeLiteralName "HallPoint") (Transformation|GetActorLocation (Variables|/Game/Blueprints/Babysitter_BP.Babysitter_BP_C|GetStartPoint (Variables|Default|GetBabysitterObject))))
  (AI|RunBehaviorTree "/Game/AI/Babysitter_BT.Babysitter_BT"))

(fn ConstructionScript)