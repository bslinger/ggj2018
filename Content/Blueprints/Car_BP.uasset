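; Car actor that moves along the spline of a referenced path actor, starting automatically at BeginPlay.
; It finds the spline component on FollowPath, prints its name and caches the spline length.
; A timeline's Distance track is scaled by that length each update to sample world-space location and rotation, which are applied to the car by teleporting the location without sweep.
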(event EventBeginPlay
  (bind _output_get (Variables|Default|SetSpllineToFollow (Actor|GetComponentbyClass (Variables|Default|GetFollowPath) "/Script/Engine.SplineComponent")))
  (Development|PrintString (Utilities|GetDisplayName _output_get))
  (Variables|Default|SetSplineLength (Spline|GetSplineLength _output_get))
  (bind _distance (Timeline|DistanceAlongSpline Play)
    (:Update
      (bind _output_get_2 (Variables|Default|SetLocationAlongSpline (Spline|GetLocationatDistanceAlongSpline (Variables|Default|GetSpllineToFollow) (* _distance (Variables|Default|GetSplineLength)) "World")))
      (Transformation|SetActorRotation (Spline|GetRotationatDistanceAlongSpline (Variables|Default|GetSpllineToFollow) (* _distance (Variables|Default|GetSplineLength)) "World"))
      (Transformation|SetActorLocation _output_get_2 false true))))

(fn ConstructionScript)