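; Stationary player that looks between three targets (door, computer, window) with Q and E, starting on the computer at BeginPlay.
; A timeline rotates the camera toward the selected target, with the index clamped at both ends.
; A second timeline zooms the FOV in once the computer is faced, reverses when switching away, and notifies Monitor_BP on finish.
; The player also registers itself with Boom_GameMode_BP.
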(event Custom|RotateCameraToPoint
  (params (Point :type Vector))
  ;[1 1 1] RotateCameraToPoint
  (bind _output_get (Variables|Default|SetCameraInitialRotation (Variables|/Script/Engine.SceneComponent|GetRelativeRotation (Variables|Default|GetCamera))))
  (bind _rotateprogression (Timeline|CameraRotationTimeline PlayFromStart)
    (:Update
      (Transformation|SetRelativeRotation (Variables|Default|GetCamera) (Math|Rotator|Lerp(Rotator) _output_get (Math|Rotator|FindLookatRotation (Transformation|GetActorLocation) Point) _rotateprogression) false false))
    (:Finished
      (if (Utilities|IsCurrentTargetComputer)
        (CallFunction|DoFOVZoom true)))))

(event Custom|DoFOVZoom
  (params (ZoomIn :type Boolean))
  ;[1 1 1] Do FOV Zoom
  (if ZoomIn
    (bind _fovzoomvalue (Timeline|FOVZoom PlayFromStart)
      (:Update
        (Camera|SetFieldOfView (Variables|Default|GetCamera) (Math|Float|Lerp (Variables|Default|GetInitial%20FOV) (Variables|Default|GetZoomedFOV) _fovzoomvalue)))
      (:Finished
        (bind _asmonitor_bp (Utilities|Casting|CastToMonitor_BP (Variables|Default|GetMonitor)))
        (Default|OnFOVFinish _asmonitor_bp ZoomIn)))
    (else
      (Timeline|FOVZoom ReverseFromEnd))))

(event EventBeginPlay
  ;[1 1 1] BeginPlay
  (Utilities|RegisterSelfwithGameMode)
  (Utilities|SetInitialFOV
    (:Out
      (Variables|Default|SetCurrentTargetIndex 1)
      (CallFunction|RotateCameratoPoint (Transformation|GetActorLocation (Variables|Default|GetComputerTarget))))))

(event Input|KeyboardEvents|Q
  (params (Key :type Key%20Structure))
  ;[1 1 1] Switch Left
  (:Pressed
    (if (Utilities|IsCurrentTargetComputer)
      (CallFunction|DoFOVZoom false))
    (bind _result (Math|Integer|DecrementInt (Variables|Default|GetCurrentTargetIndex))
      (:%20%20
        (bind _output_get (Variables|Default|SetCurrentTargetIndex (Math|Integer|Clamp(Integer) _result 0 (- (Utilities|Array|Length (Variables|Default|GetTargetPositionArray)) 1))))
        (CallFunction|RotateCameratoPoint (Transformation|GetActorLocation (Utilities|Array|Get(acopy) (Variables|Default|GetTargetPositionArray) _output_get)))))))

(event Input|KeyboardEvents|E
  (params (Key :type Key%20Structure))
  ;[1 1 1] Switch Right
  (:Pressed
    (if (Utilities|IsCurrentTargetComputer)
      (CallFunction|DoFOVZoom false))
    (bind _result (Math|Integer|IncrementInt (Variables|Default|GetCurrentTargetIndex))
      (:%20%20
        (bind _output_get (Variables|Default|SetCurrentTargetIndex (Math|Integer|Clamp(Integer) _result 0 (- (Utilities|Array|Length (Variables|Default|GetTargetPositionArray)) 1))))
        (CallFunction|RotateCameratoPoint (Transformation|GetActorLocation (Utilities|Array|Get(acopy) (Variables|Default|GetTargetPositionArray) _output_get)))))))

(fn ConstructionScript
  (bind _targetpositionarray (Variables|Default|GetTargetPositionArray))
  (Utilities|Array|SetArrayElem _targetpositionarray 0 (Variables|Default|GetDoorTarget))
  (Utilities|Array|SetArrayElem _targetpositionarray 1 (Variables|Default|GetComputerTarget))
  (Utilities|Array|SetArrayElem _targetpositionarray 2 (Variables|Default|GetWindowTarget)))