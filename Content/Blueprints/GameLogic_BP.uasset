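; GameLogic_BP is the central game-logic Blueprint, linking the player, monitor and babysitter AI in a game of downloading files without getting caught.
; On BeginPlay it registers with the babysitter's AI controller, starts a looping randomized-interval timer that triggers her, and spawns the monitor.
; It relays naughty state to the AI and prints game over if she arrives during the monitor's second widget.
; LoseState turns the player's view for babysitter losses, then shows the score screen.
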(event Custom|OnBabysitterReachRoom
  ;[1 1 1] On Babysitter Reach Room
  (if (Variables|/Game/Blueprints/Monitor_BP.Monitor_BP_C|GetOnWidget2 (Variables|Default|GetMonitor))
    (Development|PrintString "GAME OVER!!!!!")))

(event Custom|SetIsNaughty
  (params (IsNaughty :type Boolean))
  ;[1 1 1] Set Is Naughty
  (bind _output_get (Variables|Default|SetIsNaughty IsNaughty))
  (Default|SetIsNaughty (Variables|Default|GetBabysitterAIController) _output_get))

(event Custom|LoseState
  (params (LoseReason :type LoseReason%20Enum :default "NewEnumerator0"))
  (Utilities|FlowControl|Sequence
    (:then_0
      (Development|PrintString (Utilities|String|Append "In LoseState" (Utilities|String|EnumtoString LoseReason)))
      (switch Utilities|FlowControl|Switch|SwitchonLoseReason LoseReason
        (:NewEnumerator0
          (Default|LookatIndex (Variables|Default|GetPlayer)))))
    (:then_1
      (Utilities|FlowControl|Delay 5.0)
      (Utilities|ShowLoseScreen))))

(event Custom|SetConnected
  (params (Connected :type Boolean))
  ;[1 1 1] Set Connected
  (bind _output_get (Variables|Default|SetIsConnected Connected))
  (Development|PrintString (Class|KismetStringLibrary|BuildStringBool "" "Connected " _output_get)))

(event EventBeginPlay
  (Utilities|SetBabysitterAIController)
  ;[1 1 1] Set Babysitter Timer
  (Utilities|Time|SetTimerbyFunctionName 0 "TriggerBabysitter" (Math|Random|RandomFloatinRange 1.0 3.0) true)
  (Utilities|SpawnMonitor))

(fn ConstructionScript)

(fn TriggerBabysitter
  (Development|PrintString "Babysitter coming")
  (Default|TriggerBabysitter (Variables|Default|GetBabysitterAIController)))