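; Monitor actor whose screen the player can toggle between two widgets, one of which counts as "naughty".
; BeginPlay caches the widget component's original widget and creates a TestWidget2_BP as the alternate screen.
; OnFOVFinish enables player input only when zoomed in, so the Activate action works only then.
; Activate swaps the displayed widget, and SetIsNaughty stores the state and forwards it to GameLogic.
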(event Custom|OnFOVFinish
  (params (ZoomedIn :type Boolean))
  (bind _returnvalue (Game|GetPlayerController 0))
  (if ZoomedIn
    (Input|EnableInput _returnvalue)
    (else
      (Input|DisableInput _returnvalue))))

(event EventBeginPlay
  (bind _returnvalue (UserInterface|CreateWidget "/Game/Widgets/TestWidget2_BP.TestWidget2_BP_C"))
  (Variables|Default|SetWidget2 _returnvalue)
  (Variables|Default|SetWidget1 (UserInterface|GetUserWidgetObject (Variables|Default|GetWidget))))

(event Collision|EventActorBeginOverlap
  (params (OtherActor :type Actor%20Object%20Reference)))

(event EventTick
  (params (DeltaSeconds :type Float%20%28single-precision%29)))

(event Input|ActionEvents|InputActionActivate
  (params (Key :type Key%20Structure))
  (:Pressed
    (if (Variables|Default|GetOnWidget2)
      (UserInterface|SetWidget (Variables|Default|GetWidget) (Variables|Default|GetWidget1))
      (Utilities|SetIsNaughty false)
      (else
        (UserInterface|SetWidget (Variables|Default|GetWidget) (Variables|Default|GetWidget2))
        (Utilities|SetIsNaughty true)))))

(fn ConstructionScript)